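; Level 1 logic actor or script that shows the WB_Level1 widget with a fade-in, starts the Back2 media and completes once four conditions are met.
; W, A, S and D OK/Disable events toggle four booleans, each change re-running CheckOK.
; When all are true, it plays the waiting animation, opens Level2 after a short delay, resets GI_Normal and marks the first level passed.
; ToMenu triggers the widget's fade-out.
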(event `self.ReceiveBeginPlay`
  (bind _returnvalue (`|CreateWidget` "/Game/UI/WB_Level1.WB_Level1_C"))
  (set `self.Level1` _returnvalue)
  (`UserWidget.AddToViewport` _returnvalue 0)
  (message `/Game/Blueprints/InterFace/INT_UIConnection.LevelFadeIn` _returnvalue)
  (`MediaPlayer.OpenSource` (`self.MediaPlayer`) "/Game/Video/back2.back2"))

(event `/Game/Blueprints/InterFace/INT_LevelConnection.W_OK`
  (set `self.1` true)
  (bind _bool (`self.CheckOK?` :!label _label))
  (if _bool
    (message `/Game/Blueprints/InterFace/INT_UIConnection.WaitingAnimation` (`self.Level1`))
    (`KismetSystemLibrary.Delay` 0.5)
    (`GameplayStatics.OpenLevel` "Level2")
    (bind _asgi_normal (cast `/Game/Blueprints/GI_Normal` (`GameplayStatics.GetGameInstance`)))
    (`/Game/Blueprints/GI_Normal.Reset` _asgi_normal)
    (`/Game/Blueprints/GI_Normal.SetPassedLevel` _asgi_normal 0 true)))

(event `/Game/Blueprints/InterFace/INT_LevelConnection.D_OK`
  (set `self.2` true)
  (goto _label))

(event `/Game/Blueprints/InterFace/INT_LevelConnection.S_OK`
  (set `self.3` true)
  (goto _label))

(event `/Game/Blueprints/InterFace/INT_LevelConnection.A_OK`
  (set `self.4` true)
  (goto _label))

(event `/Game/Blueprints/InterFace/INT_LevelConnection.W_Disable`
  (set `self.1` false)
  (goto _label))

(event `/Game/Blueprints/InterFace/INT_LevelConnection.D_Disable`
  (set `self.2` false)
  (goto _label))

(event `/Game/Blueprints/InterFace/INT_LevelConnection.S_Disable`
  (set `self.3` false)
  (goto _label))

(event `/Game/Blueprints/InterFace/INT_LevelConnection.A_Disable`
  (set `self.4` false)
  (goto _label))

(event `/Game/Blueprints/InterFace/INT_LevelConnection.ToMenu`
  (message `/Game/Blueprints/InterFace/INT_UIConnection.LevelFadeOut` (`self.Level1`)))

(fn `CheckOK?`
  (returns (Bool :type Boolean))
  (if (`self.1`)
    (if (`self.2`)
      (if (`self.3`)
        (if (`self.4`)
          (return true))))))

(fn `UserConstructionScript`)