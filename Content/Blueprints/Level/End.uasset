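; Level Blueprint for the End level, which plays music and a media background and shows either the main menu or ending widget, based on GI_Normal's Page flag.
; The ending widget also runs FINAL after a short delay when the End flag is set.
; AOK and WOK latch two flags; once both are true, a waiting animation plays before End1 opens and the game instance is reset.
; The Disable events only re-run that check, without clearing flags.
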(event `self.ReceiveBeginPlay`
  (bind _asgi_normal (cast `/Game/Blueprints/GI_Normal` (`GameplayStatics.GetGameInstance`)))
  (`/Game/Blueprints/GI_Normal.PlayBGM` _asgi_normal "/Game/Audio/BGM/bgm.bgm")
  (set `self.Page?` (`/Game/Blueprints/GI_Normal.Page` _asgi_normal))
  (if (`self.Page?`)
    (bind _returnvalue (`|CreateWidget` "/Game/UI/WB_MainMenu.WB_MainMenu_C"))
    (set `self.1_0` _returnvalue)
    (`UserWidget.AddToViewport` _returnvalue 0)
    (`MediaPlayer.OpenSource` (`self.MediaPlayer_0`) "/Game/Video/back1.back1")
    (message `/Game/Blueprints/InterFace/INT_UIConnection.LevelFadeIn` _returnvalue)
    (else
      (bind _returnvalue_2 (`|CreateWidget` "/Game/UI/WB_End.WB_End_C"))
      (set `self.2_0` _returnvalue_2)
      (`UserWidget.AddToViewport` _returnvalue_2 0)
      (`MediaPlayer.OpenSource` (`self.MediaPlayer_0`) "/Game/Video/back1.back1")
      (message `/Game/Blueprints/InterFace/INT_UIConnection.LevelFadeIn` _returnvalue_2)
      (if (`/Game/Blueprints/GI_Normal.End?` _asgi_normal)
        (`KismetSystemLibrary.Delay` 1.5)
        (`/Game/UI/WB_End.FINAL` (`self.2_0`))))))

(event `/Game/Blueprints/InterFace/INT_LevelConnection.A_OK`
  (set `self.A` true)
  (bind _b (`self.Check` :!label _label))
  (if _b
    (message `/Game/Blueprints/InterFace/INT_UIConnection.WaitingAnimation` (`self.2_0`))
    (`KismetSystemLibrary.Delay` 3.0)
    (`GameplayStatics.OpenLevel` "End1")
    (bind _asgi_normal (cast `/Game/Blueprints/GI_Normal` (`GameplayStatics.GetGameInstance`)))
    (`/Game/Blueprints/GI_Normal.Reset` _asgi_normal)))

(event `/Game/Blueprints/InterFace/INT_LevelConnection.W_OK`
  (set `self.W` true)
  (goto _label))

(event `/Game/Blueprints/InterFace/INT_LevelConnection.W_Disable`
  (goto _label))

(event `/Game/Blueprints/InterFace/INT_LevelConnection.A_Disable`
  (goto _label))

(fn `Check`
  (returns (B :type Boolean))
  (if (`self.A`)
    (if (`self.W`)
      (return true))))

(fn `TurnPage`
  (params (B1 :type Boolean)))

(fn `UserConstructionScript`)