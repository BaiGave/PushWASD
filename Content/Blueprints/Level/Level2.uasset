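; Level 2 logic Blueprint that gates progression to Level3 on four conditions named after W, A, S and D.
; BeginPlay creates the WB_Level2 widget and triggers its fade-in message.
; OK and Disable events set or clear each flag, then re-check through CheckOKLv2.
; Once all four flags are true, the widget's waiting animation plays and Level3 opens after a short delay.
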(event `self.ReceiveBeginPlay`
  (bind _returnvalue (`|CreateWidget` "/Game/UI/WB_Level2.WB_Level2_C"))
  (set `self.Level2` _returnvalue)
  (`UserWidget.AddToViewport` _returnvalue 0)
  (message `/Game/Blueprints/InterFace/INT_UIConnection.LevelFadeIn` _returnvalue))

(event `/Game/Blueprints/InterFace/INT_LevelConnection.W_OK`
  (set `self.1` true)
  (bind _ok_ (`self.CheckOK_Lv2` :!label _label))
  (if _ok_
    (message `/Game/Blueprints/InterFace/INT_UIConnection.WaitingAnimation` (`self.Level2`))
    (`KismetSystemLibrary.Delay` 3.0)
    (`GameplayStatics.OpenLevel` "Level3")))

(event `/Game/Blueprints/InterFace/INT_LevelConnection.D_OK`
  (set `self.2` true)
  (goto _label))

(event `/Game/Blueprints/InterFace/INT_LevelConnection.S_OK`
  (set `self.3` true)
  (goto _label))

(event `/Game/Blueprints/InterFace/INT_LevelConnection.A_OK`
  (set `self.4` true)
  (goto _label))

(event `/Game/Blueprints/InterFace/INT_LevelConnection.W_Disable`
  (set `self.1` false)
  (goto _label))

(event `/Game/Blueprints/InterFace/INT_LevelConnection.D_Disable`
  (set `self.2` false)
  (goto _label))

(event `/Game/Blueprints/InterFace/INT_LevelConnection.S_Disable`
  (set `self.3` false)
  (goto _label))

(event `/Game/Blueprints/InterFace/INT_LevelConnection.A_Disable`
  (set `self.4` false)
  (goto _label))

(fn `CheckOK_Lv2`
  (returns (`OK?` :type Boolean))
  (if (`self.1`)
    (if (`self.2`)
      (if (`self.3`)
        (if (`self.4`)
          (return true))))))

(fn `UserConstructionScript`
  (`parent.UserConstructionScript`))