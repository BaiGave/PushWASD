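; End5 is the Blueprint for an ending level that closes out the game and returns to the Menu level.
; On BeginPlay it shows a WB_End2 widget with a fade-in message and opens the Back3 media source.
; AOK and WOK events set flags; once both are set, the widget plays a waiting animation, then Menu opens after a delay.
; It also resets GI_Normal and marks its GameOver and Page flags.
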(event `self.ReceiveBeginPlay`
  (bind _returnvalue (`|CreateWidget` "/Game/UI/WB_End2.WB_End2_C"))
  (set `self.End` _returnvalue)
  (`UserWidget.AddToViewport` _returnvalue 0)
  (message `/Game/Blueprints/InterFace/INT_UIConnection.LevelFadeIn` _returnvalue)
  (`MediaPlayer.OpenSource` (`self.MediaPlayer_0`) "/Game/Video/back3.back3"))

(event `/Game/Blueprints/InterFace/INT_LevelConnection.A_OK`
  (set `self.A` true)
  (bind _b (`self.Check` :!label _label))
  (if _b
    (message `/Game/Blueprints/InterFace/INT_UIConnection.WaitingAnimation` (`self.End`))
    (`KismetSystemLibrary.Delay` 3.0)
    (`GameplayStatics.OpenLevel` "Menu")
    (bind _asgi_normal (cast `/Game/Blueprints/GI_Normal` (`GameplayStatics.GetGameInstance`)))
    (`/Game/Blueprints/GI_Normal.Reset` _asgi_normal)
    (set `/Game/Blueprints/GI_Normal.GameOver` true _asgi_normal)
    (set `/Game/Blueprints/GI_Normal.Page` true _asgi_normal)))

(event `/Game/Blueprints/InterFace/INT_LevelConnection.W_OK`
  (set `self.W` true)
  (goto _label))

(event `/Game/Blueprints/InterFace/INT_LevelConnection.W_Disable`
  (goto _label))

(event `/Game/Blueprints/InterFace/INT_LevelConnection.A_Disable`
  (goto _label))

(fn `Check`
  (returns (B :type Boolean))
  (if (`self.A`)
    (if (`self.W`)
      (return true))))

(fn `TurnPage`
  (params (B1 :type Boolean)))

(fn `UserConstructionScript`)