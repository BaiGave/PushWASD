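; Level 8 script for a puzzle level that completes when all four W, A, S and D conditions are satisfied at once.
; On start it shows the WB_Level8 widget with a fade-in, opens a media source and calls Rotate twice on BP_Gamepad.
; OK and Disable events set the four flags and recheck them.
; Completion plays a waiting animation, loads Level9, then resets GI_Normal and marks the level passed.
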(event `self.ReceiveBeginPlay`
  (bind _returnvalue (`|CreateWidget` "/Game/UI/WB_Level8.WB_Level8_C"))
  (bind _output_get (set `self.Level8` _returnvalue))
  (`UserWidget.AddToViewport` _output_get 0)
  (message `/Game/Blueprints/InterFace/INT_UIConnection.LevelFadeIn` _output_get)
  (`MediaPlayer.OpenSource` (`self.MediaPlayer`) "/Game/Video/back3.back3")
  (`KismetSystemLibrary.DelayUntilNextTick`)
  (bind _returnvalue_2 (`GameplayStatics.GetActorOfClass` "/Game/Blueprints/Player/BP_Gamepad.BP_Gamepad_C"))
  (`/Game/Blueprints/Player/BP_Gamepad.Rotate` _returnvalue_2)
  (`KismetSystemLibrary.Delay` 0.01)
  (`/Game/Blueprints/Player/BP_Gamepad.Rotate` _returnvalue_2))

(event `self.W_OK`
  (set `self.1` true)
  (bind _bool (`self.CheckOK_Lv3` :!label _label))
  (if _bool
    (message `/Game/Blueprints/InterFace/INT_UIConnection.WaitingAnimation` (`self.Level8`))
    (`KismetSystemLibrary.Delay` 0.5)
    (`GameplayStatics.OpenLevel` "Level9")
    (bind _asgi_normal (cast `/Game/Blueprints/GI_Normal` (`GameplayStatics.GetGameInstance`)))
    (`/Game/Blueprints/GI_Normal.Reset` _asgi_normal)
    (`/Game/Blueprints/GI_Normal.SetPassedLevel` _asgi_normal 7 true)))

(event `self.D_OK`
  (set `self.2` true)
  (goto _label))

(event `self.S_OK`
  (set `self.3` true)
  (goto _label))

(event `self.A_OK`
  (set `self.4` true)
  (goto _label))

(event `self.W_Disable`
  (set `self.1` false)
  (goto _label))

(event `self.D_Disable`
  (set `self.2` false)
  (goto _label))

(event `self.S_Disable`
  (set `self.3` false)
  (goto _label))

(event `self.A_Disable`
  (set `self.4` false)
  (goto _label))

(event `self.ToMenu`
  (message `/Game/Blueprints/InterFace/INT_UIConnection.LevelFadeOut` (`self.Level8`)))

(fn `CheckOK_Lv3`
  (returns (Bool :type Boolean))
  (if (`self.1`)
    (if (`self.2`)
      (if (`self.3`)
        (if (`self.4`)
          (return true))))))

(fn `UserConstructionScript`
  (`parent.UserConstructionScript`))