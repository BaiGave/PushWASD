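; Level script for End2, an interlude level that shows the WB_End2 widget and moves on to End3.
; BeginPlay creates the widget, triggers its fade-in and opens the Back3 media source.
; The SOK event sets flag S, and both it and SDisable run Check, which passes when S is set.
; A pass plays the waiting animation, then after a delay opens End3 and calls Reset on GI_Normal.
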(event `self.ReceiveBeginPlay`
  (bind _returnvalue (`|CreateWidget` "/Game/UI/WB_End2.WB_End2_C"))
  (set `self.End` _returnvalue)
  (`UserWidget.AddToViewport` _returnvalue 0)
  (message `/Game/Blueprints/InterFace/INT_UIConnection.LevelFadeIn` _returnvalue)
  (`MediaPlayer.OpenSource` (`self.MediaPlayer_0`) "/Game/Video/back3.back3"))

(event `self.S_OK`
  (set `self.S` true)
  (bind _b (`self.Check` :!label _label))
  (if _b
    (message `/Game/Blueprints/InterFace/INT_UIConnection.WaitingAnimation` (`self.End`))
    (`KismetSystemLibrary.Delay` 3.0)
    (`GameplayStatics.OpenLevel` "End3")
    (bind _asgi_normal (cast `/Game/Blueprints/GI_Normal` (`GameplayStatics.GetGameInstance`)))
    (`/Game/Blueprints/GI_Normal.Reset` _asgi_normal)))

(event `self.S_Disable`
  (goto _label))

(fn `Check`
  (returns (B :type Boolean))
  (if (`self.S`)
    (return true)))

(fn `TurnPage`
  (params (B1 :type Boolean)))

(fn `UserConstructionScript`)