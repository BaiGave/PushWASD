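; Level 16 logic: shows the WB_Level16 widget with a fade-in, opens the Back6 media source, and runs a four-condition completion puzzle.
; W, D, S and A OK/Disable events set or clear four flags, each change re-running CheckOKLv3.
; When all four are true, it plays the waiting animation, opens Level17 after a delay, then resets GI_Normal.
; ToMenu triggers the widget's fade-out message.
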(event `self.ReceiveBeginPlay`
  (bind _returnvalue (`|CreateWidget` "/Game/UI/WB_Level16.WB_Level16_C"))
  (bind _output_get (set `self.Level16` _returnvalue))
  (`UserWidget.AddToViewport` _output_get 0)
  (message `/Game/Blueprints/InterFace/INT_UIConnection.LevelFadeIn` _output_get)
  (`MediaPlayer.OpenSource` (`self.MediaPlayer`) "/Game/Video/back6.back6"))

(event `self.W_OK`
  (set `self.1` true)
  (bind _bool (`self.CheckOK_Lv3` :!label _label))
  (if _bool
    (message `/Game/Blueprints/InterFace/INT_UIConnection.WaitingAnimation` (`self.Level16`))
    (`KismetSystemLibrary.Delay` 3.0)
    (`GameplayStatics.OpenLevel` "Level17")
    (bind _asgi_normal (cast `/Game/Blueprints/GI_Normal` (`GameplayStatics.GetGameInstance`)))
    (`/Game/Blueprints/GI_Normal.Reset` _asgi_normal)))

(event `self.D_OK`
  (set `self.2` true)
  (goto _label))

(event `self.S_OK`
  (set `self.3` true)
  (goto _label))

(event `self.A_OK`
  (set `self.4` true)
  (goto _label))

(event `self.W_Disable`
  (set `self.1` false)
  (goto _label))

(event `self.D_Disable`
  (set `self.2` false)
  (goto _label))

(event `self.S_Disable`
  (set `self.3` false)
  (goto _label))

(event `self.A_Disable`
  (set `self.4` false)
  (goto _label))

(event `self.ToMenu`
  (message `/Game/Blueprints/InterFace/INT_UIConnection.LevelFadeOut` (`self.Level16`)))

(fn `CheckOK_Lv3`
  (returns (Bool :type Boolean))
  (if (`self.1`)
    (if (`self.2`)
      (if (`self.3`)
        (if (`self.4`)
          (return true))))))

(fn `UserConstructionScript`
  (`parent.UserConstructionScript`))