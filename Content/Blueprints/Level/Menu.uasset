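; Menu level script that opens either the main menu or the level screen when play begins.
; On BeginPlay it starts background music through the GI_Normal game instance, then reads its Page flag to create WB_MainMenu or WB_Level.
; Both branches add the widget to the viewport, open the same background media source and trigger the widget's fade-in.
; The TurnPage function is an empty stub.
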(event `self.ReceiveBeginPlay`
  (bind _asgi_normal (cast `/Game/Blueprints/GI_Normal` (`GameplayStatics.GetGameInstance`)))
  (`/Game/Blueprints/GI_Normal.PlayBGM` _asgi_normal "/Game/Audio/BGM/bgm.bgm")
  (set `self.Page?` (`/Game/Blueprints/GI_Normal.Page` _asgi_normal))
  (if (`self.Page?`)
    (bind _returnvalue (`|CreateWidget` "/Game/UI/WB_MainMenu.WB_MainMenu_C"))
    (set `self.1` _returnvalue)
    (`UserWidget.AddToViewport` _returnvalue 0)
    (`MediaPlayer.OpenSource` (`self.MediaPlayer`) "/Game/Video/back1.back1")
    (message `/Game/Blueprints/InterFace/INT_UIConnection.LevelFadeIn` _returnvalue)
    (else
      (bind _returnvalue_2 (`|CreateWidget` "/Game/UI/WB_Level.WB_Level_C"))
      (set `self.2` _returnvalue_2)
      (`UserWidget.AddToViewport` _returnvalue_2 0)
      (`MediaPlayer.OpenSource` (`self.MediaPlayer`) "/Game/Video/back1.back1")
      (message `/Game/Blueprints/InterFace/INT_UIConnection.LevelFadeIn` _returnvalue_2))))

(fn `TurnPage`
  (params (B1 :type Boolean)))

(fn `UserConstructionScript`)