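; BP_Ctrl_3 is a Ctrl special tile that responds to BP_Block actors entering and leaving its box trigger.
; It tracks occupants in an array, playing a floor-down sound on the first press and re-arming once empty.
; A BP_A_Block press sends a Ctrl+A gamepad message, raises GINormal's CtrlBlocks and sets three sprites.
; Any exit decrements that counter; if it turns negative, a departing A block triggers the ESC message.
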(event `self.Box.OnComponentBeginOverlap`
  (params (OverlappedComponent :type "PrimitiveComponent Object Reference") (OtherActor :type "Actor Object Reference") (OtherComp :type "PrimitiveComponent Object Reference") (OtherBodyIndex :type Integer) (bFromSweep :type Boolean) (SweepResult :type "HitResult Structure (by ref)"))
  (`self.Pressed` OtherActor))

(event `self.Box.OnComponentEndOverlap`
  (params (OverlappedComponent :type "PrimitiveComponent Object Reference") (OtherActor :type "Actor Object Reference") (OtherComp :type "PrimitiveComponent Object Reference") (OtherBodyIndex :type Integer))
  (`self.Leave` OtherActor))

(fn `Leave`
  (params (Object :type "Object Object Reference"))
  (bind _blocks (`self.Blocks`))
  (bind _ctrl_blocks (`/Game/Blueprints/GI_Normal.Ctrl_Blocks` (`self.As GI Normal`)))
  (set `/Game/Blueprints/GI_Normal.Ctrl_Blocks` (- _ctrl_blocks 1) (`self.As GI Normal`))
  (if (not (>= _ctrl_blocks 0))
    ;[1 1 1] 从数组中移除离开区域的盒子
    (bind _asbp_block (cast `/Game/Blueprints/Box/BP_Block` Object))
    (if (`KismetStringLibrary.EqualEqual_StrStr` (`KismetSystemLibrary.GetDisplayName` _asbp_block) "BP_A_Block")
      (message `/Game/Blueprints/InterFace/INT_BlockMove.ESC` (`self.Gamepad`))
      (`PaperSpriteComponent.SetSprite` (`self.Sprite`) "/Game/Art/Tiles/Ctrl/ctrl_tdedge_Sprite.ctrl_tdedge_Sprite")
      (`PaperSpriteComponent.SetSprite` (`self.Sprite1`) "/Game/Art/Tiles/Switch/left_Sprite.left_Sprite")
      (`PaperSpriteComponent.SetSprite` (`self.Sprite2`) "/Game/Art/Tiles/Switch/right_Sprite.right_Sprite")))
  (bind _asbp_block_2 (cast `/Game/Blueprints/Box/BP_Block` Object))
  (if (`KismetArrayLibrary.Array_Contains` _blocks _asbp_block_2)
    (`KismetArrayLibrary.Array_RemoveItem` _blocks _asbp_block_2)
    (if (== (`KismetArrayLibrary.Array_Length` (`self.Blocks`)) 0)
      (set `self.CanIPress?` true))))

(fn `Pressed`
  (params (Object :type "Object Object Reference"))
  (bind _as_gi_normal (`self.As GI Normal`))
  (bind _blocks (`self.Blocks`))
  (bind _asbp_block (cast `/Game/Blueprints/Box/BP_Block` Object))
  (set `self.Temp_Object` _asbp_block)
  (if (not (`KismetArrayLibrary.Array_Contains` _blocks (`self.Temp_Object`)))
    (`KismetArrayLibrary.Array_Add` _blocks (`self.Temp_Object`))
    (if (`self.CanIPress?`)
      (set `self.CanIPress?` false)
      (`GameplayStatics.PlaySound2D` "/Game/Audio/floordown.floordown" 1.0 1.0 0.0 null null)
      (if (`KismetStringLibrary.EqualEqual_StrStr` (`KismetSystemLibrary.GetDisplayName` _asbp_block) "BP_A_Block")
        (message `/Game/Blueprints/InterFace/INT_BlockMove.CtrlA` (`self.Gamepad`))
        (set `/Game/Blueprints/GI_Normal.Ctrl_Blocks` (+ (`/Game/Blueprints/GI_Normal.Ctrl_Blocks` _as_gi_normal) 2) _as_gi_normal)
        (`PaperSpriteComponent.SetSprite` (`self.Sprite`) "/Game/Art/Tiles/Pressed/ctrl_tdedge_Sprite.ctrl_tdedge_Sprite")
        (`PaperSpriteComponent.SetSprite` (`self.Sprite1`) "/Game/Art/Tiles/Pressed/left_Sprite.left_Sprite")
        (`PaperSpriteComponent.SetSprite` (`self.Sprite2`) "/Game/Art/Tiles/Pressed/right_Sprite.right_Sprite")))))

(fn `UserConstructionScript`
  (`parent.UserConstructionScript`))