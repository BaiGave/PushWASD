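; BP_Swtich_LTurn1 is a special-tile switch that sends a left-rotate message to the gamepad actor when a block lands on it.
; On BeginPlay it caches the BP_Gamepad, and its Box overlap events track the BP_Block actors inside.
; A CanIPress latch fires RotateLMessage on a newly entering block, then stays locked until the last tracked block leaves.
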(event `self.ReceiveBeginPlay`
  (bind _returnvalue (`GameplayStatics.GetActorOfClass` "/Game/Blueprints/Player/BP_Gamepad.BP_Gamepad_C"))
  (set `self.Gamepad` _returnvalue))

(event `self.Box.OnComponentBeginOverlap`
  (params (OverlappedComponent :type "PrimitiveComponent Object Reference") (OtherActor :type "Actor Object Reference") (OtherComp :type "PrimitiveComponent Object Reference") (OtherBodyIndex :type Integer) (bFromSweep :type Boolean) (SweepResult :type "HitResult Structure (by ref)"))
  (bind _blocks (`self.Blocks`))
  (bind _asbp_block (cast `/Game/Blueprints/Box/BP_Block` OtherActor))
  (set `self.Temp_Object` _asbp_block)
  (if (not (`KismetArrayLibrary.Array_Contains` _blocks (`self.Temp_Object`)))
    (`KismetArrayLibrary.Array_Add` _blocks (`self.Temp_Object`))
    (if (`self.CanIPress?`)
      (set `self.CanIPress?` false)
      (message `/Game/Blueprints/InterFace/INT_BlockMove.RotateL` (`self.Gamepad`)))))

(event `self.Box.OnComponentEndOverlap`
  (params (OverlappedComponent :type "PrimitiveComponent Object Reference") (OtherActor :type "Actor Object Reference") (OtherComp :type "PrimitiveComponent Object Reference") (OtherBodyIndex :type Integer))
  (bind _blocks (`self.Blocks`))
  ;[1 1 1] 从数组中移除离开区域的盒子
  (bind _asbp_block (cast `/Game/Blueprints/Box/BP_Block` OtherActor))
  (if (`KismetArrayLibrary.Array_Contains` _blocks _asbp_block)
    (`KismetArrayLibrary.Array_RemoveItem` _blocks _asbp_block)
    (if (== (`KismetArrayLibrary.Array_Length` (`self.Blocks`)) 0)
      (set `self.CanIPress?` true))))

(fn `UserConstructionScript`
  (`parent.UserConstructionScript`))