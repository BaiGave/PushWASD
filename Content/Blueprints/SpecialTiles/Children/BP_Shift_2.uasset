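; BP_Shift_2 is a special tile Blueprint that changes its appearance while something overlaps its Box component.
; On begin overlap it switches its two sprite components to one pair of Shift sprite assets, and on end overlap it sets them to another pair.
; The overlap events do not filter the other actor, and the construction script only calls the parent.
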(event `self.Box.OnComponentBeginOverlap`
  (params (OverlappedComponent :type "PrimitiveComponent Object Reference") (OtherActor :type "Actor Object Reference") (OtherComp :type "PrimitiveComponent Object Reference") (OtherBodyIndex :type Integer) (bFromSweep :type Boolean) (SweepResult :type "HitResult Structure (by ref)"))
  (`PaperSpriteComponent.SetSprite` (`self.Sprite`) "/Game/Art/Tiles/Pressed/shift_up_Sprite.shift_up_Sprite")
  (`PaperSpriteComponent.SetSprite` (`self.Sprite1`) "/Game/Art/Tiles/Pressed/down_Sprite.down_Sprite"))

(event `self.Box.OnComponentEndOverlap`
  (params (OverlappedComponent :type "PrimitiveComponent Object Reference") (OtherActor :type "Actor Object Reference") (OtherComp :type "PrimitiveComponent Object Reference") (OtherBodyIndex :type Integer))
  (`PaperSpriteComponent.SetSprite` (`self.Sprite`) "/Game/Art/Tiles/Shift/shift_top_Sprite.shift_top_Sprite")
  (`PaperSpriteComponent.SetSprite` (`self.Sprite1`) "/Game/Art/Tiles/Shift/shift_down_Sprite.shift_down_Sprite"))

(fn `UserConstructionScript`
  (`parent.UserConstructionScript`))