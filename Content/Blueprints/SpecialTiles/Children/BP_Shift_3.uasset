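; BP_Shift_3 is a special tile Blueprint that changes its Paper2D sprites when something overlaps its Box.
; Begin and end overlap both set the Shift left/right edge and Down sprites, differing only in the third sprite, which switches between Up and Top.
; Neither handler filters the overlapping actor, and the construction script just calls the parent's.
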(event `self.Box.OnComponentBeginOverlap`
  (params (OverlappedComponent :type "PrimitiveComponent Object Reference") (OtherActor :type "Actor Object Reference") (OtherComp :type "PrimitiveComponent Object Reference") (OtherBodyIndex :type Integer) (bFromSweep :type Boolean) (SweepResult :type "HitResult Structure (by ref)"))
  (`PaperSpriteComponent.SetSprite` (`self.Sprite`) "/Game/Art/Tiles/Pressed/shift_lredge_Sprite.shift_lredge_Sprite")
  (`PaperSpriteComponent.SetSprite` (`self.Sprite1`) "/Game/Art/Tiles/Pressed/down_Sprite.down_Sprite")
  (`PaperSpriteComponent.SetSprite` (`self.Sprite2`) "/Game/Art/Tiles/Pressed/up_Sprite.up_Sprite"))

(event `self.Box.OnComponentEndOverlap`
  (params (OverlappedComponent :type "PrimitiveComponent Object Reference") (OtherActor :type "Actor Object Reference") (OtherComp :type "PrimitiveComponent Object Reference") (OtherBodyIndex :type Integer))
  (`PaperSpriteComponent.SetSprite` (`self.Sprite`) "/Game/Art/Tiles/Shift/shift_lredge_Sprite.shift_lredge_Sprite")
  (`PaperSpriteComponent.SetSprite` (`self.Sprite1`) "/Game/Art/Tiles/Switch/down_Sprite.down_Sprite")
  (`PaperSpriteComponent.SetSprite` (`self.Sprite2`) "/Game/Art/Tiles/Switch/top_Sprite.top_Sprite"))

(fn `UserConstructionScript`
  (`parent.UserConstructionScript`))