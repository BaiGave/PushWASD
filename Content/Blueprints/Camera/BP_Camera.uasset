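; Camera actor that drifts with the mouse and plays left or right spring-arm yaw rotations.
; FollowMouse starts a looping timer that offsets the actor from a fixed location by the scaled cursor distance from viewport center, clamping the Y axis.
; RotateR and RotateL lerp yaw through timelines, then chain into Rotate_Back timelines.
; A Rotating flag makes new requests wait in a delay loop until the current sequence ends.
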(event `/Game/Blueprints/InterFace/INT_Camera.FollowMouse`
  (`KismetSystemLibrary.K2_SetTimerDelegate` (delegate `FollowM`) 0.025 true))

(event `FollowM`
  (bind _returnvalue (`WidgetLayoutLibrary.GetMousePositionOnViewport`))
  (bind (_returnvalue_x _returnvalue_y) (`KismetMathLibrary.BreakVector2D` (- _returnvalue (/ (`WidgetLayoutLibrary.GetViewportSize`) (2.0 2.0)))))
  (bind (_returnvalue_x_2 _returnvalue_y_2 _returnvalue_z) (`KismetMathLibrary.BreakVector` (/ (`KismetMathLibrary.MakeVector` _returnvalue_x _returnvalue_y) (70.0 100.0 100.0))))
  (`self.K2_SetActorLocation` (+ (40.0 68.0 200.0) (`KismetMathLibrary.MakeVector` _returnvalue_x_2 (`KismetMathLibrary.MapRangeClamped` _returnvalue_y_2 -10.0 5.0 -5.0 5.0) _returnvalue_z))))

(event `/Game/Blueprints/InterFace/INT_Camera.Rotate_R`
  (if (`self.Rotating?`) :!label _label
    (`KismetSystemLibrary.Delay` 0.05)
    (goto _label)
    (else
      (set `self.R1_0` (`SceneComponent.K2_GetComponentRotation` (`self.SpringArm`)))
      (`KismetSystemLibrary.K2_SetTimerDelegate` (delegate `RotateR`) 0.05)
      (set `self.Rotating?` true))))

(event `/Game/Blueprints/InterFace/INT_Camera.Rotate_L`
  (if (`self.Rotating?`) :!label _label_2
    (`KismetSystemLibrary.Delay` 0.05)
    (goto _label_2)
    (else
      (set `self.R1` (`SceneComponent.K2_GetComponentRotation` (`self.SpringArm`)))
      (`KismetSystemLibrary.K2_SetTimerDelegate` (delegate `RotateL`) 0.05)
      (set `self.Rotating?` true))))

(event `RotateR`
  (bind (_r1_0_roll _r1_0_pitch _r1_0_yaw) (`KismetMathLibrary.BreakRotator` (`self.R1_0`)))
  (bind (_direction _movementa) (`Timeline|时间轴_0`)
    (:`Update`
      (`SceneComponent.K2_SetWorldRotation` (`self.SpringArm`) (`KismetMathLibrary.MakeRotator` _r1_0_roll _r1_0_pitch (`KismetMathLibrary.Lerp` _r1_0_yaw (+ (`self.Rotation_0`) _r1_0_yaw) _movementa)) false false))
    (:`Finished`
      (set `self.R2_0` (`SceneComponent.K2_GetComponentRotation` (`self.SpringArm`)))
      (`KismetSystemLibrary.K2_SetTimerDelegate` (delegate `Rotate_Back_R`) 0.05))))

(event `RotateL`
  (bind (_r1_roll _r1_pitch _r1_yaw) (`KismetMathLibrary.BreakRotator` (`self.R1`)))
  (bind (_direction _movementa) (`Timeline|移动`)
    (:`Update`
      (`SceneComponent.K2_SetWorldRotation` (`self.SpringArm`) (`KismetMathLibrary.MakeRotator` _r1_roll _r1_pitch (`KismetMathLibrary.Lerp` _r1_yaw (+ (`self.Rotation`) _r1_yaw) _movementa)) false false))
    (:`Finished`
      (set `self.R2` (`SceneComponent.K2_GetComponentRotation` (`self.SpringArm`)))
      (`KismetSystemLibrary.K2_SetTimerDelegate` (delegate `Rotate_Back_L`) 0.05))))

(event `Rotate_Back_R`
  (bind (_r2_0_roll _r2_0_pitch _r2_0_yaw) (`KismetMathLibrary.BreakRotator` (`self.R2_0`)))
  (bind (_direction _movementa) (`Timeline|时间轴_1` :!via `PlayFromStart`)
    (:`Update`
      (`SceneComponent.K2_SetWorldRotation` (`self.SpringArm`) (`KismetMathLibrary.MakeRotator` _r2_0_roll _r2_0_pitch (`KismetMathLibrary.Lerp` _r2_0_yaw (+ (`self.Rotation2_0`) _r2_0_yaw) _movementa)) false false))
    (:`Finished`
      (set `self.Rotating?` false))))

(event `Rotate_Back_L`
  (bind (_r2_roll _r2_pitch _r2_yaw) (`KismetMathLibrary.BreakRotator` (`self.R2`)))
  (bind (_direction _movementa) (`Timeline|时间轴` :!via `PlayFromStart`)
    (:`Update`
      (`SceneComponent.K2_SetWorldRotation` (`self.SpringArm`) (`KismetMathLibrary.MakeRotator` _r2_roll _r2_pitch (`KismetMathLibrary.Lerp` _r2_yaw (+ (`self.Rotation2`) _r2_yaw) _movementa)) false false))
    (:`Finished`
      (set `self.Rotating?` false))))

(fn `UserConstructionScript`)