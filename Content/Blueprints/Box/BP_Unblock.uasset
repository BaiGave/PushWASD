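; BP_Unblock is a Blueprint in the Box folder that looks up level and ending actors by name.
; Its Level function compares the given name through a nested branch chain covering fifteen numbered levels and six End variants.
; Each match returns the GetActorOfClass result for the corresponding class, and unmatched names have no explicit return.
; The event graph and construction script contain no active logic.
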(fn `Level`
  (params (Name :type String))
  (returns (ReturnValue :type "/Game/Blueprints/Level/Level1 Object Reference"))
  (locals (N :type String))
  (set `local.N` Name)
  (if (`KismetStringLibrary.EqualEqual_StrStr` (`local.N`) "Level1")
    (bind _returnvalue (`GameplayStatics.GetActorOfClass` "/Game/Blueprints/Level/Level1.Level1_C"))
    (return _returnvalue)
    (elif (`KismetStringLibrary.EqualEqual_StrStr` (`local.N`) "Level2")
      (bind _returnvalue_2 (`GameplayStatics.GetActorOfClass` "/Game/Blueprints/Level/Level2.Level2_C"))
      (return _returnvalue_2)
      (elif (`KismetStringLibrary.EqualEqual_StrStr` (`local.N`) "Level3")
        (bind _returnvalue_3 (`GameplayStatics.GetActorOfClass` "/Game/Blueprints/Level/Level3.Level3_C"))
        (return _returnvalue_3)
        (elif (`KismetStringLibrary.EqualEqual_StrStr` (`local.N`) "Level4")
          (bind _returnvalue_4 (`GameplayStatics.GetActorOfClass` "/Game/Blueprints/Level/Level4.Level4_C"))
          (return _returnvalue_4)
          (elif (`KismetStringLibrary.EqualEqual_StrStr` (`local.N`) "Level5")
            (bind _returnvalue_5 (`GameplayStatics.GetActorOfClass` "/Game/Blueprints/Level/Level5.Level5_C"))
            (return _returnvalue_5)
            (elif (`KismetStringLibrary.EqualEqual_StrStr` (`local.N`) "Level6")
              (bind _returnvalue_6 (`GameplayStatics.GetActorOfClass` "/Game/Blueprints/Level/Level6.Level6_C"))
              (return _returnvalue_6)
              (elif (`KismetStringLibrary.EqualEqual_StrStr` (`local.N`) "Level7")
                (bind _returnvalue_7 (`GameplayStatics.GetActorOfClass` "/Game/Blueprints/Level/Level7.Level7_C"))
                (return _returnvalue_7)
                (elif (`KismetStringLibrary.EqualEqual_StrStr` (`local.N`) "Level8")
                  (bind _returnvalue_8 (`GameplayStatics.GetActorOfClass` "/Game/Blueprints/Level/Level8.Level8_C"))
                  (return _returnvalue_8)
                  (elif (`KismetStringLibrary.EqualEqual_StrStr` (`local.N`) "Level9")
                    (bind _returnvalue_9 (`GameplayStatics.GetActorOfClass` "/Game/Blueprints/Level/Level9.Level9_C"))
                    (return _returnvalue_9)
                    (elif (`KismetStringLibrary.EqualEqual_StrStr` (`local.N`) "Level10")
                      (bind _returnvalue_10 (`GameplayStatics.GetActorOfClass` "/Game/Blueprints/Level/Level10.Level10_C"))
                      (return _returnvalue_10)
                      (elif (`KismetStringLibrary.EqualEqual_StrStr` (`local.N`) "Level11")
                        (bind _returnvalue_11 (`GameplayStatics.GetActorOfClass` "/Game/Blueprints/Level/Level11.Level11_C"))
                        (return _returnvalue_11)
                        (elif (`KismetStringLibrary.EqualEqual_StrStr` (`local.N`) "Level12")
                          (bind _returnvalue_12 (`GameplayStatics.GetActorOfClass` "/Game/Blueprints/Level/Level12.Level12_C"))
                          (return _returnvalue_12)
                          (elif (`KismetStringLibrary.EqualEqual_StrStr` (`local.N`) "Level13")
                            (bind _returnvalue_13 (`GameplayStatics.GetActorOfClass` "/Game/Blueprints/Level/Level13.Level13_C"))
                            (return _returnvalue_13)
                            (elif (`KismetStringLibrary.EqualEqual_StrStr` (`local.N`) "Level14")
                              (bind _returnvalue_14 (`GameplayStatics.GetActorOfClass` "/Game/Blueprints/Level/Level14.Level14_C"))
                              (return _returnvalue_14)
                              (elif (`KismetStringLibrary.EqualEqual_StrStr` (`local.N`) "Level15")
                                (bind _returnvalue_15 (`GameplayStatics.GetActorOfClass` "/Game/Blueprints/Level/Level15.Level15_C"))
                                (return _returnvalue_15)
                                (elif (`KismetStringLibrary.EqualEqual_StrStr` (`local.N`) "End")
                                  (bind _returnvalue_16 (`GameplayStatics.GetActorOfClass` "/Game/Blueprints/Level/End.End_C"))
                                  (return _returnvalue_16)
                                  (elif (`KismetStringLibrary.EqualEqual_StrStr` (`local.N`) "End1")
                                    (bind _returnvalue_17 (`GameplayStatics.GetActorOfClass` "/Game/Blueprints/Level/End1.End1_C"))
                                    (return _returnvalue_17)
                                    (elif (`KismetStringLibrary.EqualEqual_StrStr` (`local.N`) "End2")
                                      (bind _returnvalue_18 (`GameplayStatics.GetActorOfClass` "/Game/Blueprints/Level/End2.End2_C"))
                                      (return _returnvalue_18)
                                      (elif (`KismetStringLibrary.EqualEqual_StrStr` (`local.N`) "End3")
                                        (bind _returnvalue_19 (`GameplayStatics.GetActorOfClass` "/Game/Blueprints/Level/End3.End3_C"))
                                        (return _returnvalue_19)
                                        (elif (`KismetStringLibrary.EqualEqual_StrStr` (`local.N`) "End4")
                                          (bind _returnvalue_20 (`GameplayStatics.GetActorOfClass` "/Game/Blueprints/Level/End4.End4_C"))
                                          (return _returnvalue_20)
                                          (elif (`KismetStringLibrary.EqualEqual_StrStr` (`local.N`) "End5")
                                            (bind _returnvalue_21 (`GameplayStatics.GetActorOfClass` "/Game/Blueprints/Level/End5.End5_C"))
                                            (return _returnvalue_21)))))))))))))))))))))))

(fn `UserConstructionScript`)