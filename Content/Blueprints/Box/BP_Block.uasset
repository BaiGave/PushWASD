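; BP_Block is a Paper2D grid block that slides in 16-unit steps, singly or as moved by BP_Gamepad.
; WASD moves check the next cell with a line trace, then update a target location that a timer-driven timeline lerps toward.
; Directional traces report adjacent blocks or empty space, and TraceWASD collects unvisited neighbours for a connected-block search.
; Flipbook events briefly swap the sprite for an animation, such as reaching the goal.
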(event `self.ReceiveBeginPlay`
  ;[1 1 1 1 93] 初始化
  (set `self.Loc` (`SceneComponent.K2_GetComponentLocation` (`self.Sprite`)))
  (bind _returnvalue (`GameplayStatics.GetActorOfClass` "/Game/Blueprints/Player/BP_Gamepad.BP_Gamepad_C"))
  (set `self.Gamepad` _returnvalue))

(event `/Game/Blueprints/InterFace/INT_BlockMove.Remove_FlipBook`
  ;[1 1 1 1 71] 移除序列帧动画
  (`SceneComponent.SetVisibility` (`self.PaperFlipbook`) false false)
  (`SceneComponent.SetVisibility` (`self.Sprite`) true false))

(event `/Game/Blueprints/InterFace/INT_BlockMove.Set_FlipBook`
  (params (Flipbook :type "PaperFlipbook Object Reference"))
  ;[1 1 1 1 50] 播放到达终点动画（播放1次）
  (`PaperFlipbookComponent.SetFlipbook` (`self.PaperFlipbook`) Flipbook)
  (`SceneComponent.SetVisibility` (`self.PaperFlipbook`) true false)
  (`SceneComponent.SetVisibility` (`self.Sprite`) false false)
  (`KismetSystemLibrary.Delay` 1.0)
  (`SceneComponent.SetVisibility` (`self.PaperFlipbook`) false false)
  (`SceneComponent.SetVisibility` (`self.Sprite`) true false))

(event `Update`
  ;[1 1 1 1 50] 平滑位移A->B
  (bind (_direction _movementa) (`Timeline|SmoothMovement` :!via `PlayFromStart`)
    (:`Update`
      (`self.K2_SetActorLocation` (`KismetMathLibrary.VLerp` (`self.K2_GetActorLocation`) (`self.Loc`) _movementa) true))))

(event `/Game/Blueprints/InterFace/INT_BlockMove.MovedByGamepad`
  (params (V1 :type "Vector Structure"))
  ;[1 1 1] 整体移动
  (set `self.Loc` (+ (`self.Loc`) V1))
  (`KismetSystemLibrary.K2_SetTimerDelegate` (delegate `Update`) (`self.PreSecondCa`) true))

(event `/Game/Blueprints/InterFace/INT_BlockMove.Set_Block_Loc`
  (params (Loc :type "Vector Structure"))
  ;[1 1 1 1 34] 设置目标地点
  (set `self.Loc` (+ (`self.Loc`) Loc)))

(event `/Game/Blueprints/InterFace/INT_BlockMove.Move_WASD`
  (params (ID :type Integer))
  (switch `int` ID
    (:`0`
      ;[1 1 1 1 61] WASD平滑移动
      (bind _can_ (`self.N_CanIMoveT?`))
      (if _can_
        (set `self.Loc` (+ (`self.Loc`) (0.0 -16.0 0.0)))
        (`KismetSystemLibrary.K2_SetTimerDelegate` (delegate `Update`) (`self.PreSecondCa`) true)))
    (:`1`
      (bind _can__2 (`self.N_CanIMoveL?`))
      (if _can__2
        (set `self.Loc` (+ (`self.Loc`) (-16.0 0.0 0.0)))
        (`KismetSystemLibrary.K2_SetTimerDelegate` (delegate `Update`) (`self.PreSecondCa`) true)))
    (:`2`
      (bind _can__3 (`self.N_CanIMoveD?`))
      (if _can__3
        (set `self.Loc` (+ (`self.Loc`) (0.0 16.0 0.0)))
        (`KismetSystemLibrary.K2_SetTimerDelegate` (delegate `Update`) (`self.PreSecondCa`) true)))
    (:`3`
      (bind _can__4 (`self.N_CanIMoveR?`))
      (if _can__4
        (set `self.Loc` (+ (`self.Loc`) (16.0 0.0 0.0)))
        (`KismetSystemLibrary.K2_SetTimerDelegate` (delegate `Update`) (`self.PreSecondCa`) true)))))

(fn `Get_State`
  (params (ID :type "/Game/Blueprints/Box/BP_Block Object Reference"))
  (returns (`Upper?` :type Boolean))
  (if (`KismetStringLibrary.EqualEqual_StrStr` (`KismetSystemLibrary.GetDisplayName` ID) "BP_W_Block")
    (return (`self.Upper?`))
    (elif (`KismetStringLibrary.EqualEqual_StrStr` (`KismetSystemLibrary.GetDisplayName` ID) "BP_A_Block")
      (return (`self.Upper?`))
      (elif (`KismetStringLibrary.EqualEqual_StrStr` (`KismetSystemLibrary.GetDisplayName` ID) "BP_S_Block")
        (return (`self.Upper?`))
        (elif (`KismetStringLibrary.EqualEqual_StrStr` (`KismetSystemLibrary.GetDisplayName` ID) "BP_D_Block")
          (return (`self.Upper?`))
          (else
            (return (`self.Upper?`))))))))

(fn `N_CanIMoveD?`
  (returns (`Can？` :type Boolean))
  (bind _loc (`self.Loc`))
  (bind (_outhit _returnvalue) (`KismetSystemLibrary.LineTraceSingle` _loc (+ _loc (0.0 16.0 0.0)) "TraceTypeQuery1"))
  (return (not _returnvalue)))

(fn `N_CanIMoveL?`
  (returns (`Can？` :type Boolean))
  (bind _loc (`self.Loc`))
  (bind (_outhit _returnvalue) (`KismetSystemLibrary.LineTraceSingle` _loc (+ _loc (-16.0 0.0 0.0)) "TraceTypeQuery1"))
  (return (not _returnvalue)))

(fn `N_CanIMoveR?`
  (returns (`Can？` :type Boolean))
  (bind _loc (`self.Loc`))
  (bind (_outhit _returnvalue) (`KismetSystemLibrary.LineTraceSingle` _loc (+ _loc (16.0 0.0 0.0)) "TraceTypeQuery1"))
  (return (not _returnvalue)))

(fn `N_CanIMoveT?`
  (returns (`Can？` :type Boolean))
  (bind _loc (`self.Loc`))
  (bind (_outhit _returnvalue) (`KismetSystemLibrary.LineTraceSingle` _loc (+ _loc (0.0 -16.0 0.0)) "TraceTypeQuery1"))
  (return (not _returnvalue)))

(fn `Trace_A`
  (returns (OutHitHitActor :type "/Game/Blueprints/Box/BP_Block Object Reference") (`Air?` :type Boolean))
  (bind _loc (`self.Loc`))
  (bind (_outhit _returnvalue) (`KismetSystemLibrary.LineTraceSingle` _loc (+ _loc (-16.0 0.0 0.0)) "TraceTypeQuery1"))
  (bind _asbp_block (cast `/Game/Blueprints/Box/BP_Block` (`.HitActor` (`GameplayStatics.BreakHitResult` _outhit)))
    (:`then`
      (bind _returnvalue_2 (== _returnvalue false))
      (return _asbp_block _returnvalue_2))
    (:`CastFailed`
      (return null _returnvalue_2))))

(fn `Trace_D`
  (returns (OutHitHitActor :type "/Game/Blueprints/Box/BP_Block Object Reference") (`Air?` :type Boolean))
  (bind _loc (`self.Loc`))
  (bind (_outhit _returnvalue) (`KismetSystemLibrary.LineTraceSingle` _loc (+ _loc (16.0 0.0 0.0)) "TraceTypeQuery1"))
  (bind _asbp_block (cast `/Game/Blueprints/Box/BP_Block` (`.HitActor` (`GameplayStatics.BreakHitResult` _outhit)))
    (:`then`
      (bind _returnvalue_2 (== _returnvalue false))
      (return _asbp_block _returnvalue_2))
    (:`CastFailed`
      (return null _returnvalue_2))))

(fn `Trace_S`
  (returns (OutHitHitActor :type "/Game/Blueprints/Box/BP_Block Object Reference") (`Air?` :type Boolean))
  (bind _loc (`self.Loc`))
  (bind (_outhit _returnvalue) (`KismetSystemLibrary.LineTraceSingle` _loc (+ _loc (0.0 16.0 0.0)) "TraceTypeQuery1"))
  (bind _asbp_block (cast `/Game/Blueprints/Box/BP_Block` (`.HitActor` (`GameplayStatics.BreakHitResult` _outhit)))
    (:`then`
      (bind _returnvalue_2 (== _returnvalue false))
      (return _asbp_block _returnvalue_2))
    (:`CastFailed`
      (return null _returnvalue_2))))

(fn `Trace_SingleDir`
  (params (A :type "Array of String (by ref)") (B :type "Vector Structure"))
  (returns (Out :type "Array of String") (Out2 :type "Array of String"))
  (locals (TempArray :type "Array of String") (NextLoopArray :type "Array of String"))
  (bind _loc (`self.Loc`))
  (bind _temparray (`local.TempArray`))
  (bind _nextlooparray (`local.NextLoopArray`))
  (set `local.TempArray` A)
  (bind _outhit (`KismetSystemLibrary.LineTraceSingle` _loc (+ _loc B) "TraceTypeQuery1"))
  (bind _asbp_block (cast `/Game/Blueprints/Box/BP_Block` (`.HitActor` (`GameplayStatics.BreakHitResult` _outhit)))
    (:`then`
      (bind _returnvalue (`KismetStringLibrary.Conv_ObjectToString` _asbp_block))
      (if (== (`KismetArrayLibrary.Array_Find` _temparray _returnvalue) -1)
        (`KismetArrayLibrary.Array_Set` (`local.TempArray`) (`KismetArrayLibrary.Array_Length` _temparray) _returnvalue true)
        (`KismetArrayLibrary.Array_Set` _nextlooparray (`KismetArrayLibrary.Array_Length` _nextlooparray) _returnvalue true))
      (return (`local.TempArray`) (`local.NextLoopArray`)))
    (:`CastFailed`
      (return (`local.TempArray`)))))

(fn `Trace_W`
  (returns (OutHitHitActor :type "/Game/Blueprints/Box/BP_Block Object Reference") (`Air?` :type Boolean))
  (bind _loc (`self.Loc`))
  (bind (_outhit _returnvalue) (`KismetSystemLibrary.LineTraceSingle` _loc (+ _loc (0.0 -16.0 0.0)) "TraceTypeQuery1"))
  (bind _asbp_block (cast `/Game/Blueprints/Box/BP_Block` (`.HitActor` (`GameplayStatics.BreakHitResult` _outhit)))
    (:`then`
      (bind _returnvalue_2 (== _returnvalue false))
      (return _asbp_block _returnvalue_2))
    (:`CastFailed`
      (return null _returnvalue_2))))

(fn `TraceWASD`
  (params (Added :type "Array of String (by ref)"))
  (returns (Result :type "Array of String") (NexrLoop :type "Array of String"))
  (locals (Add :type "Array of String") (NextLoopArray :type "Array of String"))
  (set `local.Add` Added)
  (bind (_out _out2) (`self.Trace_SingleDir` (`local.Add`) (0.0 -16.0 0.0)))
  (`KismetArrayLibrary.Array_Append` (`local.NextLoopArray`) _out2)
  (bind (_out_2 _out2_2) (`self.Trace_SingleDir` _out (0.0 16.0 0.0)))
  (`KismetArrayLibrary.Array_Append` (`local.NextLoopArray`) _out2_2)
  (bind (_out_3 _out2_3) (`self.Trace_SingleDir` _out_2 (-16.0 0.0 0.0)))
  (`KismetArrayLibrary.Array_Append` (`local.NextLoopArray`) _out2_3)
  (bind (_out_4 _out2_4) (`self.Trace_SingleDir` _out_3 (16.0 0.0 0.0)))
  (`KismetArrayLibrary.Array_Append` (`local.NextLoopArray`) _out2_4)
  (return _out_4 (`local.NextLoopArray`)))

(fn `UserConstructionScript`)