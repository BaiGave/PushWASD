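; BP_A_Block is a sprite-based block that moves in 16-unit steps, apparently work in progress.
; It caches the sprite's location in Loc at BeginPlay; MoveA calls CanIMoveR and shifts Loc along -X if clear.
; CanIMoveR runs a debug-drawn Visibility line trace, but also offsets the actor unswept regardless of the result.
; The other three direction checks return false, and their branching logic is disconnected.
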(event `self.ReceiveBeginPlay`
  (set `self.Loc` (`SceneComponent.K2_GetComponentLocation` (`self.Sprite`))))

(event `/Game/Blueprints/InterFace/INT_BlockMove.Move_A`
  (bind _can_ (`self.CanIMoveR?`))
  (if _can_
    (set `self.Loc` (+ (`self.Loc`) (-16.0 0.0 0.0)))))

(fn `CanIMoveD?`
  (returns (`Can?` :type Boolean))
  (return false))

(fn `CanIMoveL?`
  (returns (`Can?` :type Boolean))
  (return false))

(fn `CanIMoveR?`
  (returns (`Can？` :type Boolean))
  (bind _loc (`self.Loc`))
  (bind (_outhits _returnvalue) (`KismetSystemLibrary.LineTraceMulti` :`Start` _loc :`End` (+ _loc (-16.0 0.0 0.0)) :`TraceChannel` "TraceTypeQuery1" :`DrawDebugType` "ForDuration"))
  (`self.K2_AddActorWorldOffset` (-16.0 0.0 0.0))
  (return (not _returnvalue)))

(fn `CanIMoveT?`
  (returns (`Can?` :type Boolean))
  (return false))

(fn `UserConstructionScript`
  (`parent.UserConstructionScript`))