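; A letter A block, a child Blueprint in the Box family, that displays as either uppercase or lowercase.
; The SetUpper and SetLower events set the Upper flag and swap the sprite to the matching A artwork.
; The construction script runs the parent's, then picks the sprite from Upper so the placed block reflects its case.
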(event `/Game/Blueprints/InterFace/INT_BlockMove.Set_Lower`
  (set `self.Upper?` false)
  (`PaperSpriteComponent.SetSprite` (`self.Sprite`) "/Game/Art/Sprites/Blocks/lowercase_a_block_Sprite.lowercase_a_block_Sprite"))

(event `/Game/Blueprints/InterFace/INT_BlockMove.Set_Upper`
  (set `self.Upper?` true)
  (`PaperSpriteComponent.SetSprite` (`self.Sprite`) "/Game/Art/Sprites/Blocks/A_block_Sprite.A_block_Sprite"))

(fn `UserConstructionScript`
  (`parent.UserConstructionScript`)
  (if (`self.Upper?`)
    (`PaperSpriteComponent.SetSprite` (`self.Sprite`) "/Game/Art/Sprites/Blocks/A_block_Sprite.A_block_Sprite")
    (else
      (`PaperSpriteComponent.SetSprite` (`self.Sprite`) "/Game/Art/Sprites/Blocks/lowercase_a_block_Sprite.lowercase_a_block_Sprite"))))