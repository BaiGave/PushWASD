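; BP_S_Unblock is a box trigger child Blueprint that reacts only to an actor whose display name is BP_S_Block.
; On overlap begin, it stops that block's message, clears its message state and calls SOKMessage on the level resolved from the current level name.
; On overlap end, it restarts the block's message, makes its own Box ignore Visibility and a custom trace channel, and calls the level's SDisableMessage.
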(event `self.Box.OnComponentBeginOverlap`
  (params (OverlappedComponent :type "PrimitiveComponent Object Reference") (OtherActor :type "Actor Object Reference") (OtherComp :type "PrimitiveComponent Object Reference") (OtherBodyIndex :type Integer) (bFromSweep :type Boolean) (SweepResult :type "HitResult Structure (by ref)"))
  (if (`KismetStringLibrary.EqualEqual_StrStr` (`KismetSystemLibrary.GetDisplayName` OtherActor) "BP_S_Block")
    (message `/Game/Blueprints/InterFace/INT_BlockMove.Stop` OtherActor)
    (message `/Game/Blueprints/InterFace/INT_BlockMove.Set_State` OtherActor false)
    (bind _returnvalue (`GameplayStatics.GetCurrentLevelName` true))
    (bind _returnvalue_2 (`self.Level` _returnvalue))
    (message `/Game/Blueprints/InterFace/INT_LevelConnection.S_OK` _returnvalue_2)))

(event `self.Box.OnComponentEndOverlap`
  (params (OverlappedComponent :type "PrimitiveComponent Object Reference") (OtherActor :type "Actor Object Reference") (OtherComp :type "PrimitiveComponent Object Reference") (OtherBodyIndex :type Integer))
  (bind _box (`self.Box`))
  (if (`KismetStringLibrary.EqualEqual_StrStr` (`KismetSystemLibrary.GetDisplayName` OtherActor) "BP_S_Block")
    (message `/Game/Blueprints/InterFace/INT_BlockMove.Start` OtherActor)
    (`PrimitiveComponent.SetCollisionResponseToChannel` _box "ECC_GameTraceChannel1" "ECR_Ignore")
    (`PrimitiveComponent.SetCollisionResponseToChannel` _box "ECC_Visibility" "ECR_Ignore")
    (bind _returnvalue (`GameplayStatics.GetCurrentLevelName` true))
    (bind _returnvalue_2 (`self.Level` _returnvalue))
    (message `/Game/Blueprints/InterFace/INT_LevelConnection.S_Disable` _returnvalue_2)))

(fn `UserConstructionScript`
  (`parent.UserConstructionScript`))