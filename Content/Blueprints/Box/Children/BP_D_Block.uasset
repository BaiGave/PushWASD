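; BP_D_Block is a letter D block, a child Blueprint that shows either an uppercase or lowercase D sprite.
; The SetUpper and SetLower events set the Upper flag and swap the sprite to match.
; The construction script runs the parent's script, then picks the sprite from Upper, so the chosen case shows when the block is constructed.
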(event `/Game/Blueprints/InterFace/INT_BlockMove.Set_Lower`
  (set `self.Upper?` false)
  (`PaperSpriteComponent.SetSprite` (`self.Sprite`) "/Game/Art/Sprites/Blocks/lowercase_d_block_Sprite.lowercase_d_block_Sprite"))

(event `/Game/Blueprints/InterFace/INT_BlockMove.Set_Upper`
  (set `self.Upper?` true)
  (`PaperSpriteComponent.SetSprite` (`self.Sprite`) "/Game/Art/Sprites/Blocks/D_block_Sprite.D_block_Sprite"))

(fn `UserConstructionScript`
  (`parent.UserConstructionScript`)
  (if (`self.Upper?`)
    (`PaperSpriteComponent.SetSprite` (`self.Sprite`) "/Game/Art/Sprites/Blocks/D_block_Sprite.D_block_Sprite")
    (else
      (`PaperSpriteComponent.SetSprite` (`self.Sprite`) "/Game/Art/Sprites/Blocks/lowercase_d_block_Sprite.lowercase_d_block_Sprite"))))