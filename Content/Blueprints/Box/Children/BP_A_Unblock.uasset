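; BP_A_Unblock is a child box Blueprint for the letter A target that reacts to BP_A_Block, matched by display name.
; Its construction script picks the uppercase or lowercase sprite from the Upper flag.
; On overlap, a block with matching case triggers the level's A-OK message and gets a matching flipbook message.
; When overlap ends, it restarts the block's message, ignores two collision channels, disables the level message and removes the flipbook.
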(event `self.Box.OnComponentBeginOverlap`
  (params (OverlappedComponent :type "PrimitiveComponent Object Reference") (OtherActor :type "Actor Object Reference") (OtherComp :type "PrimitiveComponent Object Reference") (OtherBodyIndex :type Integer) (bFromSweep :type Boolean) (SweepResult :type "HitResult Structure (by ref)"))
  (if (`KismetStringLibrary.EqualEqual_StrStr` (`KismetSystemLibrary.GetDisplayName` OtherActor) "BP_A_Block")
    (bind _asbp_block (cast `/Game/Blueprints/Box/BP_Block` OtherActor))
    (bind _upper_ (message `/Game/Blueprints/InterFace/INT_BlockMove.Get_State` _asbp_block _asbp_block))
    (if (== _upper_ (`self.Upper?`))
      (bind _returnvalue (`GameplayStatics.GetCurrentLevelName` true))
      (bind _returnvalue_2 (`self.Level` _returnvalue))
      (message `/Game/Blueprints/InterFace/INT_LevelConnection.A_OK` _returnvalue_2)
      (if (`self.Upper?`)
        (message `/Game/Blueprints/InterFace/INT_BlockMove.Set_FlipBook` _asbp_block "/Game/Art/Animations/A_OK1.A_OK1")
        (else
          (message `/Game/Blueprints/InterFace/INT_BlockMove.Set_FlipBook` _asbp_block "/Game/Art/Animations/lowa1.lowa1"))))))

(event `self.Box.OnComponentEndOverlap`
  (params (OverlappedComponent :type "PrimitiveComponent Object Reference") (OtherActor :type "Actor Object Reference") (OtherComp :type "PrimitiveComponent Object Reference") (OtherBodyIndex :type Integer))
  (bind _box (`self.Box`))
  (if (`KismetStringLibrary.EqualEqual_StrStr` (`KismetSystemLibrary.GetDisplayName` OtherActor) "BP_A_Block")
    (message `/Game/Blueprints/InterFace/INT_BlockMove.Start` OtherActor)
    (`PrimitiveComponent.SetCollisionResponseToChannel` _box "ECC_GameTraceChannel1" "ECR_Ignore")
    (`PrimitiveComponent.SetCollisionResponseToChannel` _box "ECC_Visibility" "ECR_Ignore")
    (bind _returnvalue (`GameplayStatics.GetCurrentLevelName` true))
    (bind _returnvalue_2 (`self.Level` _returnvalue))
    (message `/Game/Blueprints/InterFace/INT_LevelConnection.A_Disable` _returnvalue_2)
    (message `/Game/Blueprints/InterFace/INT_BlockMove.Remove_FlipBook` OtherActor)))

(fn `UserConstructionScript`
  (`parent.UserConstructionScript`)
  (if (`self.Upper?`)
    (`PaperSpriteComponent.SetSprite` (`self.Sprite`) "/Game/Art/Sprites/Blocks/A_unblock_Sprite.A_unblock_Sprite")
    (else
      (`PaperSpriteComponent.SetSprite` (`self.Sprite`) "/Game/Art/Sprites/Blocks/lowercase_a_unblock_Sprite.lowercase_a_unblock_Sprite"))))